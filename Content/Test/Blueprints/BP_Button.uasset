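; Test button that fills a progress bar through repeated presses and fires ProgressbarIsFull once when it reaches the maximum.
; Presses come from the HMDLocomotionPawn's interact dispatcher or from overlaps with Sphere1, re-armed when an overlap ends.
; Each press adds progress and, below the maximum, restarts a looping timer that drains it.
; Progressbar's RepNotify updates the text render and prints the value.
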(event `self.ReceiveBeginPlay`
  (bind _ashmdlocomotion_pawn (cast `/Game/VirtualRealityBP/Blueprints/HMDLocomotionPawn` (`GameplayStatics.GetPlayerPawn` 0)))
  (add `/Game/VirtualRealityBP/Blueprints/HMDLocomotionPawn.D_Interact` _ashmdlocomotion_pawn (delegate `Interact`)))

(event `Interact`
  (`KismetSystemLibrary.K2_ClearAndInvalidateTimerHandle` (`self.DecreaseTimer`) :!label _label)
  (bind _output_get (set `self.Progressbar` (`KismetMathLibrary.FMin` (+ (`self.Progressbar`) (`self.AddPerPress`)) 100.0)))
  (if (>= _output_get (`self.ProgressMax`))
    (`/Engine/EditorBlueprintResources/StandardMacros.DoOnce` false
      (:`Completed`
        (`self.ProgressbarIsFull`)))
    (else
      (bind _returnvalue (`KismetSystemLibrary.K2_SetTimer` null "Decrease" (`self.DecreaseDelay`) true))
      (set `self.DecreaseTimer` _returnvalue))))

(event `self.Sphere1.OnComponentBeginOverlap`
  (params (OverlappedComponent :type "PrimitiveComponent Object Reference") (OtherActor :type "Actor Object Reference") (OtherComp :type "PrimitiveComponent Object Reference") (OtherBodyIndex :type Integer) (bFromSweep :type Boolean) (SweepResult :type "HitResult Structure (by ref)"))
  (`/Engine/EditorBlueprintResources/StandardMacros.DoOnce` false :!label _label_2
    (:`Completed`
      (goto _label))))

(event `self.Sphere1.OnComponentEndOverlap`
  (params (OverlappedComponent :type "PrimitiveComponent Object Reference") (OtherActor :type "Actor Object Reference") (OtherComp :type "PrimitiveComponent Object Reference") (OtherBodyIndex :type Integer))
  (goto _label_2 :!via `Reset`))

(fn `Decrease`
  (if (> (`self.Progressbar`) 0.0)
    (set `self.Progressbar` (`KismetMathLibrary.FMax` (- (`self.Progressbar`) (`self.DecreaseValue`))))))

(fn `OnRep_Progressbar`
  (bind _progressbar (`self.Progressbar`))
  (`TextRenderComponent.K2_SetText` (`self.TextRender`) (`KismetTextLibrary.Conv_DoubleToText` _progressbar "HalfToEven"))
  (`KismetSystemLibrary.PrintString` (`KismetStringLibrary.Conv_DoubleToString` _progressbar)))

(fn `UserConstructionScript`)