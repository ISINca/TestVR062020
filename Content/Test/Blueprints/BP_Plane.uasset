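; BP_Plane is a test actor that rises when a starter button's progress bar fills, then starts a video.
; BeginPlay binds UpPlane to the StarterButtom progress-full event, and UpPlane starts a fast looping timer on SetWorldOffset.
; Each tick of that timer nudges the actor upward until its root reaches a fixed world height, then clears the timer and opens the test video source on the MediaPlayer.
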(event `self.ReceiveBeginPlay`
  (add `/Game/Test/Blueprints/BP_Button.ProgressbarIsFull` (`self.StarterButtom`) (delegate `UpPlane`)))

(event `UpPlane`
  (bind _returnvalue (`KismetSystemLibrary.K2_SetTimer` null "SetWorldOffset" 0.02 true))
  (set `self.UpTimer` _returnvalue))

(fn `PlayVideo`
  (`MediaPlayer.OpenSource` (`self.MediaPlayer`) "/Game/Test/Media/RV_VideoTest.RV_VideoTest"))

(fn `SetWorldOffset`
  (bind (_returnvalue_x _returnvalue_y _returnvalue_z) (`KismetMathLibrary.BreakVector` (`SceneComponent.K2_GetComponentLocation` (`self.DefaultSceneRoot`))))
  (if (< _returnvalue_z 400.0)
    (`self.K2_AddActorWorldOffset` (`KismetMathLibrary.MakeVector` 0.0 0.0 (`self.UpPerDelay`)))
    (else
      (`KismetSystemLibrary.K2_ClearAndInvalidateTimerHandle` (`self.UpTimer`))
      (`self.PlayVideo`))))

(fn `UserConstructionScript`)